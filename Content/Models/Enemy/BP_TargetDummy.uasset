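; BP_TargetDummy is a target dummy enemy actor that can take damage and be killed.
; It forwards damage, instant-kill and max-health events to its BPCDamgeSystem component, and polls that component's IsDead on Tick to destroy itself.
; It always reports itself as an enemy, exposes boss status through a Boss variable, and its Heal function does nothing but return false.
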(event EventBeginPlay)

(event Collision|EventActorBeginOverlap
  (params (OtherActor :type Actor%20Object%20Reference)))

(event EventTick
  (params (DeltaSeconds :type Float%20%28single-precision%29))
  (if (Variables|/Game/FirstPerson/Components/BPC_DamgeSystem.BPC_DamgeSystem_C|GetIsDead (Variables|Default|GetBPC_DamgeSystem))
    (Actor|DestroyActor)))

(event EventInstantKill
  (Default|InstantKill (Variables|Default|GetBPC_DamgeSystem)))

(event EventSetMaxHealth
  (params (MaxHealth :type Float%20%28double-precision%29))
  (Class|BPIDamagable|SetMaxHealth(Message) (Variables|Default|GetBPC_DamgeSystem) MaxHealth))

(event EventDoDamage
  (params (Damage :type Float%20%28double-precision%29))
  (Default|DoDamage (Variables|Default|GetBPC_DamgeSystem) Damage))

(fn ConstructionScript)

(fn Heal
  (params (Amount :type Float%20%28double-precision%29))
  (return false))

(fn IsBoss
  (return (Variables|Default|GetBoss)))

(fn IsEnemy
  (return true))